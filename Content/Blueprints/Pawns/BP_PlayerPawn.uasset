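; Player pawn that rolls a physics sphere around the level and restarts the level when it takes damage.
; ForwardBack and LeftRight axis inputs share one torque call on the sphere root, scaled by a strength variable and applied as an acceleration change.
; Any damage runs the Restart Level macro, which fades the camera out, waits for the fade, then reopens the current level by name.
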(event `InputAxis|ForwardBack`
  (params (AxisValue :type "Float (single-precision)"))
  (`PrimitiveComponent.AddTorqueInRadians` (`self.SphereRoot`) (`KismetMathLibrary.MakeVector` (* (stale `InputAxis|LeftRight` AxisValue) (`self.TorqueStrenght`)) (* AxisValue (`self.TorqueStrenght`))) "None" true :!label _label))

(event `InputAxis|LeftRight`
  (params (AxisValue :type "Float (single-precision)"))
  (goto _label))

(event `self.ReceiveAnyDamage`
  (params (Damage :type "Float (single-precision)") (DamageType :type "DamageType Object Reference") (InstigatedBy :type "Controller Object Reference") (DamageCauser :type "Actor Object Reference"))
  (`self.Restart Level`))

(fn `UserConstructionScript`)