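; BP_Cannon is a cannon actor that automatically and repeatedly fires BP_Projectile actors.
; Tick enters a Delay set by Firerate, after which a projectile spawns at the Arrow component's location and rotation, scaled by ProjectileScale.
; A timeline then animates the barrel's relative Y location, and its Finished output loops back into the Delay for the next shot.
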(event `self.ReceiveTick`
  (params (DeltaSeconds :type "Float (single-precision)"))
  (`KismetSystemLibrary.Delay` (`self.Firerate`) :!label _label)
  (`self.SpawnProjectile`)
  (bind (_direction _cannonbarrellocation) (`Timeline|Cannon Fire Timeline` :!via `PlayFromStart`)
    (:`Update`
      (`self.CannonLocationAnimation` _cannonbarrellocation))
    (:`Finished`
      (goto _label))))

(fn `CannonLocationAnimation`
  (params (NewLocation_Y :type "Float (double-precision)"))
  (`SceneComponent.K2_SetRelativeLocation` (`self.CannonBarrel`) (`KismetMathLibrary.MakeVector` 0.0 NewLocation_Y) false false))

(fn `SpawnProjectile`
  (bind _arrow (`self.Arrow`))
  (`|SpawnActorFromClass` "/Game/Blueprints/Actors/Projectiles/BP_Projectile.BP_Projectile_C" (`KismetMathLibrary.MakeTransform` (`SceneComponent.K2_GetComponentLocation` _arrow) (`SceneComponent.K2_GetComponentRotation` _arrow) (`KismetMathLibrary.Conv_DoubleToVector` (`self.ProjectileScale`))) "Undefined" "OverrideRootScale" null null))

(fn `UserConstructionScript`)