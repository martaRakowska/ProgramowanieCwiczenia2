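; BP_WinVolume is a level-exit trigger that lets the player advance once no crystals remain in the level.
; When the player overlaps its Box, it counts BP_Crystal actors and prints a message if any are left.
; Otherwise it finds the current level name in LevelList, then either opens the next entry after a short delay or quits the game on the last one.
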(event `self.Box.OnComponentBeginOverlap`
  (params (OverlappedComponent :type "PrimitiveComponent Object Reference") (OtherActor :type "Actor Object Reference") (OtherComp :type "PrimitiveComponent Object Reference") (OtherBodyIndex :type Integer) (bFromSweep :type Boolean) (SweepResult :type "HitResult Structure (by ref)"))
  (`/Game/Blueprints/Libraries/ML_Actors.IsPlayer?` OtherActor
    (:`IsPlayer`
      (if (`self.CheckAnyCrystals`)
        (if (`self.IsFinalLvl?`)
          (`KismetSystemLibrary.QuitGame` null "Quit")
          (else
            (`KismetSystemLibrary.Delay` 2.0)
            (`self.LoadNextLevel`)))
        (else
          (`KismetSystemLibrary.PrintString` "There are still crystals left!"))))))

(fn `CheckAnyCrystals`
  (returns (NoCrystalsLeft :type Boolean))
  (bind _outactors (`GameplayStatics.GetAllActorsOfClass` "/Game/Blueprints/Actors/Collectables/BP_Crystal.BP_Crystal_C"))
  (return (== (`KismetArrayLibrary.Array_Length` _outactors) 0)))

(fn `GetCurrentLevelIndex`
  (returns (NewParam :type Integer))
  (bind _returnvalue (`GameplayStatics.GetCurrentLevelName` true))
  (return (`KismetArrayLibrary.Array_Find` (`self.LevelList`) (`KismetStringLibrary.Conv_StringToName` _returnvalue))))

(fn `IsFinalLvl?`
  (returns (IsFinalLvl :type Boolean))
  (return (== (`self.GetCurrentLevelIndex`) (`KismetArrayLibrary.Array_LastIndex` (`self.LevelList`)))))

(fn `LoadNextLevel`
  (`GameplayStatics.OpenLevel` (`|GetArrayItem` (`self.LevelList`) (+ (`self.GetCurrentLevelIndex`) 1))))

(fn `UserConstructionScript`)